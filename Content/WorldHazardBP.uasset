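; World hazard actor that deals repeated damage to the player while they stand inside its sphere.
; On sphere overlap with a CharacterBP, it stores the player and calls CalculateAndApplyDamageToPlayer immediately with the configured amount and type.
; A Delay-based loop repeats the damage at DamageRate intervals while PlayerInHazard is set.
; End overlap by the stored player clears that flag, stopping the loop at its next check.
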(event `self.Sphere.OnComponentBeginOverlap`
  (params (OverlappedComponent :type "PrimitiveComponent Object Reference") (OtherActor :type "Actor Object Reference") (OtherComp :type "PrimitiveComponent Object Reference") (OtherBodyIndex :type Integer) (bFromSweep :type Boolean) (SweepResult :type "HitResult Structure (by ref)"))
  (if (== (`GameplayStatics.GetObjectClass` OtherActor) "/Game/CharacterBP.CharacterBP_C")
    (bind _ascharacter_bp (cast `/Game/CharacterBP` OtherActor))
    (bind _output_get (set `self.Player Ref` _ascharacter_bp))
    (set `self.PlayerInHazard` true)
    (`/Game/PlayerDamage.Calculate and Apply Damage to Player` _output_get (`self.Damage Amount`) (`self.Damage Type`) :!label _label)
    (`KismetSystemLibrary.Delay` (`self.Damage Rate`))
    (if (`self.PlayerInHazard`)
      (goto _label))))

(event `self.Sphere.OnComponentEndOverlap`
  (params (OverlappedComponent :type "PrimitiveComponent Object Reference") (OtherActor :type "Actor Object Reference") (OtherComp :type "PrimitiveComponent Object Reference") (OtherBodyIndex :type Integer))
  (if (== OtherActor (`self.Player Ref`))
    (set `self.PlayerInHazard` false)))

(fn `UserConstructionScript`)