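; Player character for an RPG, with axis movement, gear-based stats, regeneration and basic XP leveling.
; CalculateStats sums ten gear slots, adding base values for pools and regen.
; A Delay on Tick regenerates health, mana and stamina about every second, at 20% rate in combat; the stamina cap mistakenly checks CurrentHealth.
; X grants test XP and F equips test head gear; EquipGear handles only Head, and LevelUp just resets XP and prints.
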(event `self.ReceiveBeginPlay`
  (bind (_my_gear_head _my_gear_shoulders _my_gear_arm _my_gear_chest _my_gear_waist _my_gear_legs _my_gear_feet _my_gear_back _my_gear_mainhand _my_gear_offhand) (break `/Game/GearList` (`self.My Gear`)))
  (set `self.Head Gear` _my_gear_head)
  (set `self.Shoulder Gear` _my_gear_shoulders)
  (set `self.Arm Gear` _my_gear_arm)
  (set `self.Chest Gear` _my_gear_chest)
  (set `self.Waist Gear` _my_gear_waist)
  (set `self.Legs Gear` _my_gear_legs)
  (set `self.Feet Gear` _my_gear_feet)
  (set `self.Back Gear` _my_gear_back)
  (set `self.Main Hand Weapon` _my_gear_mainhand)
  (set `self.Off Hand Weapon` _my_gear_offhand)
  (`self.Calculate Stats`))

(event `self.ReceiveTick`
  (params (DeltaSeconds :type "Float (single-precision)"))
  (`|ExecutionSequence`
    (:`then_0`
      (`KismetSystemLibrary.Delay` 1.0)
      (`self.Health_Regen`)
      (`self.Mana_Regen`)
      (`self.Stammina_Regen`))))

(event `Death`)

(event `InputAxis|MoveY`
  (params (AxisValue :type "Float (single-precision)"))
  ;[1 1 1] Movement / Controls
  (`self.AddMovementInput` (`KismetMathLibrary.GetForwardVector` (`self.K2_GetActorRotation`)) AxisValue))

(event `InputAxis|MoveX`
  (params (AxisValue :type "Float (single-precision)"))
  ;[1 1 1] Movement / Controls
  (`self.AddMovementInput` (`KismetMathLibrary.GetRightVector` (`self.K2_GetActorRotation`)) AxisValue))

(event `InputAxis|Rotate`
  (params (AxisValue :type "Float (single-precision)"))
  ;[1 1 1] Movement / Controls
  (`self.AddControllerYawInput` AxisValue))

(event `Key|X`
  (params (Key :type "Key Structure"))
  (:`Released`
    (`self.XP Gain` 5)))

(event `Key|F`
  (params (Key :type "Key Structure"))
  (:`Released`
    (`self.Equip Gear` (make `/Game/GearStats` 0.0 0.0 0.0 0.0 0.0 0.0 0.0 100.0 0.0 0.0 0.0 0.0 0.0 0 "None" "Head"))
    (`self.Calculate Stats`)))

(fn `Calculate Stats`
  (bind (_head_gear_armor _head_gear_magearmor _head_gear_attackdamage _head_gear_magicdamage _head_gear_critchance _head_gear_speed _head_gear_weight _head_gear_health _head_gear_mana _head_gear_stamina _head_gear_hpregen _head_gear_manaregen _head_gear_staminaregen _head_gear_gearscore) (break `/Game/GearStats` (`self.Head Gear`)))
  (bind (_shoulder_gear_armor _shoulder_gear_magearmor _shoulder_gear_attackdamage _shoulder_gear_magicdamage _shoulder_gear_critchance _shoulder_gear_speed _shoulder_gear_weight _shoulder_gear_health _shoulder_gear_mana _shoulder_gear_stamina _shoulder_gear_hpregen _shoulder_gear_manaregen _shoulder_gear_staminaregen _shoulder_gear_gearscore) (break `/Game/GearStats` (`self.Shoulder Gear`)))
  (bind (_arm_gear_armor _arm_gear_magearmor _arm_gear_attackdamage _arm_gear_magicdamage _arm_gear_critchance _arm_gear_speed _arm_gear_weight _arm_gear_health _arm_gear_mana _arm_gear_stamina _arm_gear_hpregen _arm_gear_manaregen _arm_gear_staminaregen _arm_gear_gearscore) (break `/Game/GearStats` (`self.Arm Gear`)))
  (bind (_chest_gear_armor _chest_gear_magearmor _chest_gear_attackdamage _chest_gear_magicdamage _chest_gear_critchance _chest_gear_speed _chest_gear_weight _chest_gear_health _chest_gear_mana _chest_gear_stamina _chest_gear_hpregen _chest_gear_manaregen _chest_gear_staminaregen _chest_gear_gearscore) (break `/Game/GearStats` (`self.Chest Gear`)))
  (bind (_waist_gear_armor _waist_gear_magearmor _waist_gear_attackdamage _waist_gear_magicdamage _waist_gear_critchance _waist_gear_speed _waist_gear_weight _waist_gear_health _waist_gear_mana _waist_gear_stamina _waist_gear_hpregen _waist_gear_manaregen _waist_gear_staminaregen _waist_gear_gearscore) (break `/Game/GearStats` (`self.Waist Gear`)))
  (bind (_legs_gear_armor _legs_gear_magearmor _legs_gear_attackdamage _legs_gear_magicdamage _legs_gear_critchance _legs_gear_speed _legs_gear_weight _legs_gear_health _legs_gear_mana _legs_gear_stamina _legs_gear_hpregen _legs_gear_manaregen _legs_gear_staminaregen _legs_gear_gearscore) (break `/Game/GearStats` (`self.Legs Gear`)))
  (bind (_feet_gear_armor _feet_gear_magearmor _feet_gear_attackdamage _feet_gear_magicdamage _feet_gear_critchance _feet_gear_speed _feet_gear_weight _feet_gear_health _feet_gear_mana _feet_gear_stamina _feet_gear_hpregen _feet_gear_manaregen _feet_gear_staminaregen _feet_gear_gearscore) (break `/Game/GearStats` (`self.Feet Gear`)))
  (bind (_back_gear_armor _back_gear_magearmor _back_gear_attackdamage _back_gear_magicdamage _back_gear_critchance _back_gear_speed _back_gear_weight _back_gear_health _back_gear_mana _back_gear_stamina _back_gear_hpregen _back_gear_manaregen _back_gear_staminaregen _back_gear_gearscore) (break `/Game/GearStats` (`self.Back Gear`)))
  (bind (_main_hand_weapon_armor _main_hand_weapon_magearmor _main_hand_weapon_attackdamage _main_hand_weapon_magicdamage _main_hand_weapon_critchance _main_hand_weapon_speed _main_hand_weapon_weight _main_hand_weapon_health _main_hand_weapon_mana _main_hand_weapon_stamina _main_hand_weapon_hpregen _main_hand_weapon_manaregen _main_hand_weapon_staminaregen _main_hand_weapon_gearscore) (break `/Game/GearStats` (`self.Main Hand Weapon`)))
  (bind (_off_hand_weapon_armor _off_hand_weapon_magearmor _off_hand_weapon_attackdamage _off_hand_weapon_magicdamage _off_hand_weapon_critchance _off_hand_weapon_speed _off_hand_weapon_weight _off_hand_weapon_health _off_hand_weapon_mana _off_hand_weapon_stamina _off_hand_weapon_hpregen _off_hand_weapon_manaregen _off_hand_weapon_staminaregen _off_hand_weapon_gearscore) (break `/Game/GearStats` (`self.Off Hand Weapon`)))
  (set `self.Max Health` (`KismetMathLibrary.Conv_Int64ToInt` (`KismetMathLibrary.FFloor64` (+ (`KismetMathLibrary.Conv_IntToDouble` (`self.Base Max Health`)) _head_gear_health _shoulder_gear_health _arm_gear_health _chest_gear_health _waist_gear_health _legs_gear_health _feet_gear_health _back_gear_health _main_hand_weapon_health _off_hand_weapon_health))))
  (set `self.Max Mana` (`KismetMathLibrary.FTrunc` (+ (`KismetMathLibrary.Conv_IntToDouble` (`self.Base Max Mana`)) _head_gear_mana _shoulder_gear_mana _arm_gear_mana _chest_gear_mana _waist_gear_mana _legs_gear_mana _feet_gear_mana _back_gear_mana _main_hand_weapon_mana _off_hand_weapon_mana)))
  (set `self.Max Stamina` (`KismetMathLibrary.FTrunc` (+ (`KismetMathLibrary.Conv_IntToDouble` (`self.Base Max Stamina`)) _head_gear_stamina _shoulder_gear_stamina _arm_gear_stamina _chest_gear_stamina _waist_gear_stamina _legs_gear_stamina _feet_gear_stamina _back_gear_stamina _main_hand_weapon_stamina _off_hand_weapon_stamina)))
  (set `self.Health Regen` (+ (`self.Base HP Regen`) _head_gear_hpregen _shoulder_gear_hpregen _arm_gear_hpregen _chest_gear_hpregen _waist_gear_hpregen _legs_gear_hpregen _feet_gear_hpregen _back_gear_hpregen _main_hand_weapon_hpregen _off_hand_weapon_hpregen))
  (set `self.Mana Regen` (+ (`self.Base Mana Regen`) _head_gear_manaregen _shoulder_gear_manaregen _arm_gear_manaregen _chest_gear_manaregen _waist_gear_manaregen _legs_gear_manaregen _feet_gear_manaregen _back_gear_manaregen _main_hand_weapon_manaregen _off_hand_weapon_manaregen))
  (set `self.Stamina Regen` (+ (`self.Base Stamina Regen`) _head_gear_staminaregen _shoulder_gear_staminaregen _arm_gear_staminaregen _chest_gear_staminaregen _waist_gear_staminaregen _legs_gear_staminaregen _feet_gear_staminaregen _back_gear_staminaregen _main_hand_weapon_staminaregen _off_hand_weapon_staminaregen))
  (set `self.Armor` (`KismetMathLibrary.FTrunc` (+ (`KismetMathLibrary.Conv_IntToDouble` 0) _head_gear_armor _shoulder_gear_armor _arm_gear_armor _chest_gear_armor _waist_gear_armor _legs_gear_armor _feet_gear_armor _back_gear_armor _main_hand_weapon_armor _off_hand_weapon_armor)))
  (set `self.Mage Armor` (`KismetMathLibrary.FTrunc` (+ (`KismetMathLibrary.Conv_IntToDouble` 0) _head_gear_magearmor _shoulder_gear_magearmor _arm_gear_magearmor _chest_gear_magearmor _waist_gear_magearmor _legs_gear_magearmor _feet_gear_magearmor _back_gear_magearmor _main_hand_weapon_magearmor _off_hand_weapon_magearmor)))
  (set `self.Attack Damage` (+ (`KismetMathLibrary.Conv_IntToDouble` 0) _head_gear_attackdamage _shoulder_gear_attackdamage _arm_gear_attackdamage _chest_gear_attackdamage _waist_gear_attackdamage _legs_gear_attackdamage _feet_gear_attackdamage _back_gear_attackdamage _main_hand_weapon_attackdamage _off_hand_weapon_attackdamage))
  (set `self.Magic Damage` (+ (`KismetMathLibrary.Conv_IntToDouble` 0) _head_gear_magicdamage _shoulder_gear_magicdamage _arm_gear_magicdamage _chest_gear_magicdamage _waist_gear_magicdamage _legs_gear_magicdamage _feet_gear_magicdamage _back_gear_magicdamage _main_hand_weapon_magicdamage _off_hand_weapon_magicdamage))
  (set `self.Crit Chance` (+ (`KismetMathLibrary.Conv_IntToDouble` 0) _head_gear_critchance _shoulder_gear_critchance _arm_gear_critchance _chest_gear_critchance _waist_gear_critchance _legs_gear_critchance _feet_gear_critchance _back_gear_critchance _main_hand_weapon_critchance _off_hand_weapon_critchance))
  (set `self.Weight` (+ (`KismetMathLibrary.Conv_IntToDouble` 0) _head_gear_weight _shoulder_gear_weight _arm_gear_weight _chest_gear_weight _waist_gear_weight _legs_gear_weight _feet_gear_weight _back_gear_weight _main_hand_weapon_weight _off_hand_weapon_weight))
  (set `self.Speed` (+ (`KismetMathLibrary.Conv_IntToDouble` 0) _head_gear_speed _shoulder_gear_speed _arm_gear_speed _chest_gear_speed _waist_gear_speed _legs_gear_speed _feet_gear_speed _back_gear_speed _main_hand_weapon_speed _off_hand_weapon_speed))
  (set `self.Gear Score` (+ _head_gear_gearscore _shoulder_gear_gearscore _arm_gear_gearscore _chest_gear_gearscore _waist_gear_gearscore _legs_gear_gearscore _feet_gear_gearscore _back_gear_gearscore _main_hand_weapon_gearscore _off_hand_weapon_gearscore 0)))

(fn `Equip Gear`
  (params (`Gear Being Equipped` :type "/Game/GearStats Structure"))
  (locals (`Gear Item` :type "/Game/GearStats Structure"))
  (bind _output_get (set `local.Gear Item` `Gear Being Equipped`))
  (switch `string` (`.Slot_44_94EB3E6A46B30C92572069B039F4E95A` (break `/Game/GearStats` _output_get))
    (:`Head`
      (set `self.Head Gear` (`local.Gear Item`)))))

(fn `Health_Regen`
  (bind _returnvalue (`KismetMathLibrary.Conv_IntToDouble` (`self.Max Health`)))
  (if (`self.InCombat`)
    ;[1 1 1] Health regen in combat (80% effectiveness)
    (set `self.Current Health` (+ (`self.Current Health`) (* (`self.Health Regen`) 0.2)))
    (else
      ;[1 1 1] Normal Regen
      (set `self.Current Health` (+ (`self.Current Health`) (`self.Health Regen`)))))
  ;[1 1 1] Prevent health from going over the max
  (if (> (`self.Current Health`) _returnvalue)
    (set `self.Current Health` _returnvalue))
  (`KismetSystemLibrary.PrintString` (`KismetStringLibrary.Conv_DoubleToString` (`self.Current Health`)) true false))

(fn `Level Up`
  (set `self.Current XP` 0)
  (`KismetSystemLibrary.PrintString` "Congratulations! You've Leveled up!"))

(fn `Mana_Regen`
  (bind _returnvalue (`KismetMathLibrary.Conv_IntToDouble` (`self.Max Mana`)))
  (if (`self.InCombat`)
    ;[1 1 1] Mana regen in combat (80% effectiveness)
    (set `self.Current Mana` (+ (`self.Current Mana`) (* (`self.Mana Regen`) 0.2)))
    (else
      ;[1 1 1] Normal Mana Regen
      (set `self.Current Mana` (+ (`self.Current Mana`) (`self.Mana Regen`)))))
  ;[1 1 1] Prevent mana from going over the max
  (if (> (`self.Current Mana`) _returnvalue)
    (set `self.Current Mana` _returnvalue)))

(fn `Stammina_Regen`
  (bind _returnvalue (`KismetMathLibrary.Conv_IntToDouble` (`self.Max Stamina`)))
  (if (`self.InCombat`)
    ;[1 1 1] Stamina regen in combat (80% effectiveness)
    (set `self.Current Stamina` (+ (`self.Current Stamina`) (* (`self.Stamina Regen`) 0.2)))
    (else
      ;[1 1 1] Normal Stamina Regen
      (set `self.Current Stamina` (+ (`self.Current Stamina`) (`self.Stamina Regen`)))))
  ;[1 1 1] Prevent Stamina from going over the max
  (if (> (`self.Current Health`) _returnvalue)
    (set `self.Current Stamina` _returnvalue)))

(fn `UserConstructionScript`)

(fn `XP Gain`
  (params (`XP amount` :type Integer))
  (bind _output_get (set `self.Current XP` (+ `XP amount` (`self.Current XP`))))
  (if (>= _output_get (`self.XP for next level`))
    (`self.Level Up`)))