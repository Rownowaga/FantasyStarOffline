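; WorldHealBP is a placeable heal zone that repeatedly heals the player character while they stand inside it.
; On HealZone overlap, an exact class check for CaseyCharacterBP stores the player, sets an in-zone flag and prints a debug "Hello" for any actor.
; A Delay-driven loop calls CalculatePlayerHeal with HealAmount immediately, then every HealRate seconds until end overlap clears the flag.
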(event `self.Heal Zone.OnComponentBeginOverlap`
  (params (OverlappedComponent :type "PrimitiveComponent Object Reference") (OtherActor :type "Actor Object Reference") (OtherComp :type "PrimitiveComponent Object Reference") (OtherBodyIndex :type Integer) (bFromSweep :type Boolean) (SweepResult :type "HitResult Structure (by ref)"))
  (`KismetSystemLibrary.PrintString` "Hello")
  (if (== (`GameplayStatics.GetObjectClass` OtherActor) "/Game/CaseyCharacterBP.CaseyCharacterBP_C")
    (bind _ascharacter_bp (cast `/Game/CaseyCharacterBP` OtherActor))
    (bind _output_get (set `self.Player Ref` _ascharacter_bp))
    (set `self.Player In Heal Zone` true)
    (`/Game/PlayerHeal.Calculate Player Heal` (`self.Heal Amount`) _output_get :!label _label)
    (`KismetSystemLibrary.Delay` (`self.Heal Rate`))
    (if (`self.Player In Heal Zone`)
      (goto _label))))

(event `self.Heal Zone.OnComponentEndOverlap`
  (params (OverlappedComponent :type "PrimitiveComponent Object Reference") (OtherActor :type "Actor Object Reference") (OtherComp :type "PrimitiveComponent Object Reference") (OtherBodyIndex :type Integer))
  (if (== OtherActor (`self.Player Ref`))
    (set `self.Player In Heal Zone` false)))

(fn `UserConstructionScript`)